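; BP_SoccerController is a player controller that handles movement and look input for the soccer game.
; Move_Forward and Move_Left axes move the controlled pawn along forward and right vectors built from control yaw only, so pitch does not affect movement.
; Turn_Right and Pitch_Up axes add yaw and pitch input scaled by TurnRate and frame delta time for frame-rate-independent turning.
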(event `InputAxis|Move_Forward`
  (params (AxisValue :type "Float (single-precision)"))
  (bind _returnvalue (`self.K2_GetPawn`))
  (`/Engine/EditorBlueprintResources/StandardMacros.IsValid` _returnvalue
    (:`Is Valid`
      (`Pawn.AddMovementInput` _returnvalue (`KismetMathLibrary.GetForwardVector` (`KismetMathLibrary.MakeRotator` 0.0 0.0 (.yaw (`self.GetControlRotation`)))) AxisValue false))))

(event `InputAxis|Move_Left`
  (params (AxisValue :type "Float (single-precision)"))
  (bind _returnvalue (`self.K2_GetPawn`))
  (`/Engine/EditorBlueprintResources/StandardMacros.IsValid` _returnvalue
    (:`Is Valid`
      (`Pawn.AddMovementInput` _returnvalue (`KismetMathLibrary.GetRightVector` (`KismetMathLibrary.MakeRotator` 0.0 0.0 (.yaw (`self.GetControlRotation`)))) AxisValue false))))

(event `InputAxis|Turn_Right`
  (params (AxisValue :type "Float (single-precision)"))
  (`self.AddYawInput` (* AxisValue (`GameplayStatics.GetWorldDeltaSeconds`) (`self.Turn Rate`))))

(event `InputAxis|Pitch_Up`
  (params (AxisValue :type "Float (single-precision)"))
  (`self.AddPitchInput` (* AxisValue (`GameplayStatics.GetWorldDeltaSeconds`) (`self.Turn Rate`))))

(fn `UserConstructionScript`)